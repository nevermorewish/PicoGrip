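; BP_PickupSphere is a physics sphere that can be picked up and dropped by a hand mesh and reports a fixed grip type.
; Pickup disables physics and snaps the root to the hand's CubeSocket, while Drop detaches it and re-enables physics.
; A dynamic material created at BeginPlay drives the outline through a Glow parameter, though switching it off writes to "None", so Glow is never cleared.
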(event `self.ReceiveBeginPlay`
  (bind _sphere (`self.Sphere`))
  (bind _returnvalue (`PrimitiveComponent.CreateDynamicMaterialInstance` _sphere 0 (`PrimitiveComponent.GetMaterial` _sphere 0) "None"))
  (set `self.Material` _returnvalue))

(event `/Game/Blueprints/PickupActorInterface.ToggleOutline`
  (params (ShowOutline :type Boolean))
  (bind _material (`self.Material`))
  (if ShowOutline
    (`MaterialInstanceDynamic.SetScalarParameterValue` _material "Glow" 1.0)
    (else
      (`MaterialInstanceDynamic.SetScalarParameterValue` _material "None" 0.0))))

(event `/Game/Blueprints/PickupActorInterface.Pickup`
  (params (AttachTo :type "SceneComponent Object Reference") (HandMesh :type "SceneComponent Object Reference") (HandType :type "EControllerHand Enum" :default "Left") (FlipSocket :type Boolean))
  (`PrimitiveComponent.SetSimulatePhysics` (`self.Sphere`) false)
  (`SceneComponent.K2_AttachToComponent` (`self.RootComponent`) HandMesh "CubeSocket" "SnapToTarget" "SnapToTarget" "KeepWorld" false))

(event `/Game/Blueprints/PickupActorInterface.Drop`
  (`PrimitiveComponent.SetSimulatePhysics` (`self.Sphere`) true)
  (`self.K2_DetachFromActor` "KeepWorld" "KeepWorld" "KeepWorld"))

(fn `GetGripType`
  (returns (GripType :type "/Game/Blueprints/Enum/GripType Enum"))
  (return "NewEnumerator1"))

(fn `UserConstructionScript`)
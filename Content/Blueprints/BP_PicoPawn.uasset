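; BP_PicoPawn is a Pico VR pawn with floor-level tracking that manages hand actors for the motion controllers.
; UpdateController runs shortly after BeginPlay and on device connection changes, spawning and attaching a BP_Hand to CameraScene for each connected controller.
; Right grip grabs and releases through the hand actor, and right trigger starts a gravity grab.
; Delayed teleport logic exists, but its only callers here are unreachable.
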(event `self.ReceiveEndPlay`
  (params (EndPlayReason :type "EEndPlayReason Enum" :default "Destroyed"))
  (bind _returnvalue (`PicoXRHMDFunctionLibrary.PXR_GetEventManager`))
  (clear `PicoXREventManager.DeviceConnectChangedDelegate` _returnvalue))

(event `self.ReceiveBeginPlay`
  (`|ExecutionSequence`
    (:`then_0`
      (`HeadMountedDisplayFunctionLibrary.SetTrackingOrigin` "Floor"))
    (:`then_1`
      (bind _returnvalue (`PicoXRHMDFunctionLibrary.PXR_GetEventManager`))
      (add `PicoXREventManager.DeviceConnectChangedDelegate` _returnvalue (delegate `ConnectChanged`)))
    (:`then_2`
      (`KismetSystemLibrary.Delay` 0.2)
      (`self.UpdateController`))))

(event `ConnectChanged`
  (params (Handness :type Integer) (State :type Integer))
  (`self.UpdateController`))

(event `UpdateController`
  (bind _returnvalue (`KismetMathLibrary.MakeTransform` (0.0 0.0 0.0)))
  (bind _leftcontroller (`self.LeftController`))
  (bind _rightcontroller (`self.RightController`))
  (bind _camerascene (`self.CameraScene`))
  (`|ExecutionSequence`
    (:`then_0`
      (bind _status (`PicoXRInputFunctionLibrary.PXR_GetControllerConnectionState` "LeftHand"))
      (if _status
        (`/Engine/EditorBlueprintResources/StandardMacros.IsValid` _leftcontroller
          (:`Is Not Valid`
            (bind _returnvalue_2 (`|SpawnActorFromClass` "/Game/Blueprints/BP_Hand.BP_Hand_C" _returnvalue "AlwaysSpawn" "OverrideRootScale" self "Left" null))
            (bind _output_get (set `self.LeftController` _returnvalue_2))
            (`self.K2_AttachToComponent` _output_get _camerascene "None" "SnapToTarget" "SnapToTarget" "KeepWorld" true)
            (`KismetSystemLibrary.PrintString` "Spawn Left Controller!")))
        (else
          (`/Engine/EditorBlueprintResources/StandardMacros.IsValid` _leftcontroller
            (:`Is Valid`
              (`self.K2_DestroyActor`))))))
    (:`then_1`
      (bind _status_2 (`PicoXRInputFunctionLibrary.PXR_GetControllerConnectionState` "RightHand"))
      (if _status_2
        (`/Engine/EditorBlueprintResources/StandardMacros.IsValid` _rightcontroller
          (:`Is Not Valid`
            (bind _returnvalue_3 (`|SpawnActorFromClass` "/Game/Blueprints/BP_Hand.BP_Hand_C" _returnvalue "AlwaysSpawn" "OverrideRootScale" self "Right" null))
            (bind _output_get_2 (set `self.RightController` _returnvalue_3))
            (`self.K2_AttachToComponent` _output_get_2 _camerascene "None" "SnapToTarget" "SnapToTarget" "KeepWorld" true)
            (`KismetSystemLibrary.PrintString` "Spawn Right Controller!")))
        (else
          (`/Engine/EditorBlueprintResources/StandardMacros.IsValid` _rightcontroller
            (:`Is Valid`
              (`self.K2_DestroyActor`))))))))

(event `InputAction|GripLeft`
  (params (Key :type "Key Structure")))

(event `InputAction|GripRight`
  (params (Key :type "Key Structure"))
  (bind _rightcontroller (`self.RightController`))
  (:`Pressed`
    (`/Game/Blueprints/BP_Hand.GrabActor` _rightcontroller)
    (`KismetSystemLibrary.PrintString` "PressGripRight"))
  (:`Released`
    (`/Game/Blueprints/BP_Hand.ReleaseActor` _rightcontroller)
    (`KismetSystemLibrary.PrintString` "ReleaseGripRight")))

(event `InputAction|ThumbstickLeft`
  (params (Key :type "Key Structure")))

(event `InputAction|ThumbstickRight`
  (params (Key :type "Key Structure")))

(event `InputAction|TriggerRight`
  (params (Key :type "Key Structure"))
  (:`Pressed`
    (`/Game/Blueprints/BP_Hand.Do Gravity Grab` (`self.RightController`))))

(event `InputAction|TriggerLeft`
  (params (Key :type "Key Structure")))

(event `ExecuteTeleportation`
  (params (MotionController :type "/Game/Blueprints/BP_Hand Object Reference"))
  (bind (_location _rotation) (`/Game/Blueprints/BP_Hand.GetTeleportDestination` MotionController))
  (if (`self.IsTeleporting`)
    _
    (elif (`/Game/Blueprints/BP_Hand.IsValidTeleportDestination` MotionController)
      (set `self.IsTeleporting` true)
      (`KismetSystemLibrary.Delay` (`self.FadeOutDuration`))
      (`/Game/Blueprints/BP_Hand.DisableTeleporter` MotionController)
      (`self.K2_TeleportTo` _location _rotation)
      (set `self.IsTeleporting` false)
      (else
        (`/Game/Blueprints/BP_Hand.DisableTeleporter` MotionController)))))

(fn `UserConstructionScript`)
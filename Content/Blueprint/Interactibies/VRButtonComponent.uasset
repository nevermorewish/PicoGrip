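; VR button component that an overlapping component physically pushes along a configurable axis.
; Begin overlap captures the toucher and enables Tick, which turns its movement into clamped depth and moves the button.
; ButtonPress flips state and fires a change event once per touch past engage depth, with a cooldown.
; On release the button snaps to rest, or to engaged depth for one latching type, then stops ticking.
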(event `self.ReceiveBeginPlay`
  (add `self.OnComponentEndOverlap` (delegate `OnOverlapEnd`))
  (add `self.OnComponentBeginOverlap` (delegate `OnOverlapBegin`)))

(event `OnOverlapBegin` :!signature `self.OnComponentBeginOverlap`
  (params (OverlappedComponent :type "PrimitiveComponent Object Reference") (OtherActor :type "Actor Object Reference") (OtherComp :type "PrimitiveComponent Object Reference") (OtherBodyIndex :type Integer) (bFromSweep :type Boolean) (SweepResult :type "HitResult Structure (by ref)"))
  (if (`self.bIsEnabled`)
    (`/Engine/EditorBlueprintResources/StandardMacros.IsValid` (`self.LocalInteractingComponent`)
      (:`Is Not Valid`
        (set `self.LocalInteractingComponent` OtherComp)
        (bind _output_get (set `self.OriginalBaseTransform` (`self.K2_GetComponentToWorld`)))
        (set `self.InitialLocation` (`KismetMathLibrary.InverseTransformLocation` _output_get (`self.K2_GetComponentLocation` (`self.LocalInteractingComponent`))))
        (set `self.InitialComponentLoc` (`KismetMathLibrary.InverseTransformLocation` _output_get (`self.K2_GetComponentLocation`)))
        (set `self.bToggledThisTouch` false)
        (`self.SetComponentTickEnabled` true)
        (`self.OnButtonBeginInteraction` null)))))

(event `OnOverlapEnd` :!signature `self.OnComponentEndOverlap`
  (params (OverlappedComponent :type "PrimitiveComponent Object Reference") (OtherActor :type "Actor Object Reference") (OtherComp :type "PrimitiveComponent Object Reference") (OtherBodyIndex :type Integer))
  (`/Engine/EditorBlueprintResources/StandardMacros.IsValid` (`self.LocalInteractingComponent`)
    (:`Is Valid`
      (set `self.LocalInteractingComponent` null))))

(event `self.ReceiveTick`
  (params (DeltaSeconds :type "Float (single-precision)"))
  (bind _outvec (`self.GetTargetRelativeLocation`))
  (bind _returnvalue (`self.K2_GetComponentLocation` (`self.LocalInteractingComponent`)))
  (bind _axis (`self.GetAxisValue` _returnvalue))
  (`/Engine/EditorBlueprintResources/StandardMacros.IsValid` (`self.LocalInteractingComponent`)
    (:`Is Valid`
      (if (`self.bIsEnabled`)
        (bind _output_get (set `self.OriginalBaseTransform` (`self.K2_GetComponentToWorld`)))
        (if (> (`KismetMathLibrary.Abs` (- _axis (`self.LastAxis`))) 1.0)
          (set `self.LastAxis` _axis)
          (bind _output_get_2 (set `self.CheckDepth` (`self.CheckClampDepth` (`self.InitialLocation`) (`KismetMathLibrary.InverseTransformLocation` _output_get _returnvalue))))
          (`KismetSystemLibrary.PrintString` (`KismetStringLibrary.Concat_StrStr` "CheckDepth " (`KismetStringLibrary.Conv_DoubleToString` _output_get_2)))
          (if (> _output_get_2 0.0)
            (bind _output_get_3 (set `self.New Depth` (`KismetMathLibrary.FClamp` (- (`self.GetAxisValue` (`self.InitialComponentLoc`)) (`self.CheckDepth`)) (* (`self.DepressDistance`) -1.0) (`self.GetMaxDepth`))))
            (bind _returnvalue_2 (`KismetMathLibrary.TransformLocation` (`self.InitialRelativeTransform`) (`self.SetAxisValue` _output_get_3)))
            (`self.K2_SetRelativeLocation` _returnvalue_2)
            (`KismetSystemLibrary.PrintString` (`KismetStringLibrary.Concat_StrStr` "SetLocation " (`KismetStringLibrary.Conv_DoubleToString` (`self.GetAxisValue` _returnvalue_2))))
            (`self.ButtonPress` _output_get_3 (`GameplayStatics.GetRealTimeSeconds`))))
        (else
          (set `self.LocalInteractingComponent` null))))
    (:`Is Not Valid`
      (if (== (.location (`self.GetRelativeTransform`)) _outvec :`ErrorTolerance` 0.01)
        (`self.SetComponentTickEnabled` false)
        (`self.OnButtonBeginInteraction` (`self.LocalLastInteractingActor`) (`self.LocalInteractingComponent`))
        (set `self.LocalInteractingComponent` null)
        (else
          (`self.K2_SetRelativeLocation` _outvec))))))

(fn `ButtonPress`
  (params (NewDepth :type "Float (double-precision)") (WorldTime :type "Float (double-precision)"))
  (if (and (<= NewDepth (* (`self.ButtonEngageDepth`) -1.0)) (not (`self.bToggledThisTouch`)) (>= (- WorldTime (`self.LastToggleTime`)) (`self.MinTimeBetweenEngaging`)))
    (set `self.LastToggleTime` WorldTime)
    (set `self.bToggledThisTouch` true)
    (bind _output_get (set `self.bButtonState` (not (`self.bButtonState`))))
    (`self.OnButtonStateChanged` _output_get (`self.LocalLastInteractingActor`) (`self.LocalInteractingComponent`))))

(fn `CheckClampDepth`
  (params (StartPos :type "Vector Structure") (EndPos :type "Vector Structure"))
  (returns (Depth :type "Float (double-precision)"))
  (return (`KismetMathLibrary.FClamp` (- (`self.GetAxisValue` StartPos) (`self.GetAxisValue` EndPos)) 0.0 (`self.DepressDistance`))))

(fn `GetAxisValue`
  (params (Pos :type "Vector Structure"))
  (returns (axis :type "Float (double-precision)"))
  (switch `/Game/Blueprint/Interactibies/EVRInteractibleAxis` (`self.ButtonAxis`)
    (:`NewEnumerator0`
      (return (.x Pos)))
    (:`NewEnumerator1`
      (return (.y Pos)))
    (:`NewEnumerator2`
      (return (.z Pos)))))

(fn `GetMaxDepth`
  (returns (Depth :type "Float (double-precision)"))
  (if (and (`|EnumEquality` (`self.ButtonType`) "NewEnumerator2") (`self.bButtonState`))
    (return (* (`self.ButtonEngageDepth`) -1.0))
    (else
      (return 0.0))))

(fn `GetTargetRelativeLocation`
  (returns (OutVec :type "Vector Structure"))
  (if (and (`|EnumEquality` (`self.ButtonType`) "NewEnumerator2") (`self.bButtonState`))
    (return (`KismetMathLibrary.TransformLocation` (`self.InitialRelativeTransform`) (`self.SetAxisValue` (* (`self.ButtonEngageDepth`) -1.0))))
    (else
      (return (.location (`self.InitialRelativeTransform`))))))

(fn `IsButtonUse`
  (returns (bUse :type Boolean))
  (return false))

(fn `ResetButtonLocation`)

(fn `SetAxisValue`
  (params (Value :type "Float (double-precision)"))
  (returns (Vec :type "Vector Structure"))
  (switch `/Game/Blueprint/Interactibies/EVRInteractibleAxis` (`self.ButtonAxis`)
    (:`NewEnumerator0`
      (return (`KismetMathLibrary.MakeVector` Value)))
    (:`NewEnumerator1`
      (return (`KismetMathLibrary.MakeVector` 0.0 Value)))
    (:`NewEnumerator2`
      (return (`KismetMathLibrary.MakeVector` 0.0 0.0 Value)))))
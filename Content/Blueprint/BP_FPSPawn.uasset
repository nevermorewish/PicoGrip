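; First-person pawn that carries two BP_Hand actors and supports mouse-look style axis input, movement and teleportation.
; On BeginPlay it sets a floor tracking origin, then spawns both hands and attaches them to the camera at fixed offsets, mirroring the left with negative scale.
; Axis inputs drive controller yaw, pitch and actor-relative movement.
; ExecuteTeleportation waits for the fade-out duration without drawing a fade, then moves the pawn to the hand's valid destination, raised vertically.
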(event `self.ReceiveBeginPlay`
  (bind _camera (`self.Camera`))
  (`|ExecutionSequence`
    (:`then_0`
      (`HeadMountedDisplayFunctionLibrary.SetTrackingOrigin` "Floor"))
    (:`then_1`
      (bind _returnvalue (`|SpawnActorFromClass` "/Game/VRTemplate/Blueprints/BP_Hand.BP_Hand_C" (`KismetMathLibrary.MakeTransform` (0.0 0.0 0.0)) "AlwaysSpawn" "OverrideRootScale" self "Left" null))
      (bind _output_get (set `self.LeftController` _returnvalue))
      (`self.K2_AttachToComponent` _output_get _camera "None" "SnapToTarget" "SnapToTarget" "KeepWorld" true)
      (`self.K2_AddActorLocalTransform` _output_get (`KismetMathLibrary.MakeTransform` (60.0 -30.0 0.0) (struct :`Roll` 90.0) (1.0 1.0 -1.0)) false false))
    (:`then_2`
      (bind _returnvalue_2 (`|SpawnActorFromClass` "/Game/VRTemplate/Blueprints/BP_Hand.BP_Hand_C" (`KismetMathLibrary.MakeTransform` (0.0 0.0 0.0)) "AlwaysSpawn" "OverrideRootScale" self "Right" null))
      (bind _output_get_2 (set `self.RightController` _returnvalue_2))
      (`self.K2_AttachToComponent` _output_get_2 _camera "None" "SnapToTarget" "SnapToTarget" "KeepWorld" true)
      (`self.K2_AddActorLocalTransform` _output_get_2 (`KismetMathLibrary.MakeTransform` (60.0 30.0 0.0) (struct :`Roll` 90.0)) false false))))

(event `InputAxis|Turn`
  (params (AxisValue :type "Float (single-precision)"))
  (`self.AddControllerYawInput` AxisValue))

(event `InputAxis|LookUp`
  (params (AxisValue :type "Float (single-precision)"))
  (`self.AddControllerPitchInput` AxisValue))

(event `InputAxis|MoveForward`
  (params (AxisValue :type "Float (single-precision)"))
  (`self.AddMovementInput` (`self.GetActorForwardVector`) AxisValue))

(event `InputAxis|MoveRight`
  (params (AxisValue :type "Float (single-precision)"))
  (`self.AddMovementInput` (`self.GetActorRightVector`) AxisValue))

(event `self.ExecuteTeleportation`
  (params (MotionController :type "/Game/VRTemplate/Blueprints/BP_Hand Object Reference"))
  (bind (_location _rotation) (`/Game/VRTemplate/Blueprints/BP_Hand.GetTeleportDestination` MotionController))
  (if (`self.IsTeleporting`)
    _
    (elif (`/Game/VRTemplate/Blueprints/BP_Hand.IsValidTeleportDestination` MotionController)
      (set `self.IsTeleporting` true)
      (`KismetSystemLibrary.Delay` (`self.FadeOutDuration`))
      (`/Game/VRTemplate/Blueprints/BP_Hand.DisableTeleporter` MotionController)
      (`self.K2_TeleportTo` (+ _location (0.0 0.0 100.0)) _rotation)
      (set `self.IsTeleporting` false)
      (else
        (`/Game/VRTemplate/Blueprints/BP_Hand.DisableTeleporter` MotionController)))))

(fn `UserConstructionScript`
  (`parent.UserConstructionScript`))